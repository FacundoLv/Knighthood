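; BP_KnighthoodCharacter is the player character Blueprint, managing UI, difficulty-based stats and a sword.
; On BeginPlay it creates the HUD, hidden pause and game-over widgets, then sets health and mana from the game instance's difficulty.
; Pause input toggles the menu, cursor, input mode and game pause, while GameOverEvent shows the game-over screen once and pauses.
; The child-actor weapon gets the character as owner in construction and is exposed as a BaseSword.
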(event Custom|GameOverEvent
  (bind _returnvalue (Game|GetPlayerController 0))
  (bind _gameover (Variables|Default|GetGameOver))
  ;[1 1 1] Game Over display logic
  (Utilities|FlowControl|DoOnce false
    (:Completed
      (Widget|SetVisibility _gameover "Visible")
      (Variables|/Script/Engine.PlayerController|SetbShowMouseCursor _returnvalue true)
      (Input|SetInputModeUIOnly _returnvalue _gameover "DoNotLock")
      (Game|SetGamePaused true))))

(event EventBeginPlay
  (CallFunction|CreatePauseMenu)
  (CallFunction|CreatePlayerHUD)
  (CallFunction|CreateGameOver)
  (CallFunction|SetupPlayer))

(event EventGetDamaged
  (params (DamageAmount :type Float%20%28single-precision%29))
  (Class|KnighthoodCharacter|GetDamage DamageAmount))

(event Input|ActionEvents|InputActionPause
  (params (Key :type Key%20Structure :default "None"))
  (bind _returnvalue (Game|GetPlayerController 0))
  (bind _pausemenu (Variables|Default|GetPauseMenu))
  ;[1 1 1] PauseBehaviour
  (:Pressed
    (if (Game|IsGamePaused)
      (Widget|SetVisibility _pausemenu "Collapsed")
      (Variables|/Script/Engine.PlayerController|SetbShowMouseCursor _returnvalue false)
      (Input|SetInputModeGameOnly _returnvalue)
      (Game|SetGamePaused false)
      (else
        (Widget|SetVisibility _pausemenu "Visible")
        (Variables|/Script/Engine.PlayerController|SetbShowMouseCursor _returnvalue true)
        (Input|SetInputModeGameandUI _returnvalue _pausemenu "DoNotLock" false)
        (Game|SetGamePaused true)))))

(fn ConstructionScript
  (CallFunction|SetChildWeapon))

(fn CreatePauseMenu
  (bind _returnvalue (UserInterface|CreateWidget "/Game/MyBlueprints/UI/PauseMenu.PauseMenu_C" (Game|GetPlayerController 0)))
  (bind _output_get (Variables|Default|SetPauseMenu _returnvalue))
  (UserInterface|Viewport|AddtoViewport _output_get 0)
  (Widget|SetVisibility _returnvalue "Collapsed"))

(fn CreatePlayerHUD
  (bind _returnvalue (UserInterface|CreateWidget "/Game/MyBlueprints/UI/HUD.HUD_C" (Game|GetPlayerController 0)))
  (bind _output_get (Variables|Default|SetHUD _returnvalue))
  (UserInterface|Viewport|AddtoViewport _output_get 0))

(fn CreateGameOver
  (bind _returnvalue (UserInterface|CreateWidget "/Game/MyBlueprints/UI/GameOver.GameOver_C" (Game|GetPlayerController 0)))
  (bind _output_get (Variables|Default|SetGameOver _returnvalue))
  (UserInterface|Viewport|AddtoViewport _output_get 0)
  (Widget|SetVisibility _returnvalue "Collapsed"))

(fn SetChildWeapon
  (Actor|SetOwner (Variables|/Script/Engine.ChildActorComponent|GetChildActor (Variables|Default|GetWeapon)) self))

(fn SetupPlayer
  (bind _asknighthood_game_instance (Utilities|Casting|CastToKnighthoodGameInstance (Game|GetGameInstance)))
  (switch Utilities|FlowControl|Switch|SwitchonGameDifficulty (Variables|/Game/MyBlueprints/KnighthoodGameInstance.KnighthoodGameInstance_C|GetCurrentDifficulty _asknighthood_game_instance)
    (:NewEnumerator0
      (bind _output_get (Variables|Default|SetMAX_HEALTH 3e+02))
      (Variables|Default|Sethealth _output_get)
      (bind _output_get_2 (Variables|Default|SetMAX_MANA 1.5e+02))
      (Variables|Default|Setmana _output_get_2))
    (:NewEnumerator1
      (bind _output_get_3 (Variables|Default|SetMAX_HEALTH 2e+02))
      (Variables|Default|Sethealth _output_get_3)
      (bind _output_get_4 (Variables|Default|SetMAX_MANA 1e+02))
      (Variables|Default|Setmana _output_get_4))
    (:NewEnumerator2
      (bind _output_get_5 (Variables|Default|SetMAX_HEALTH 2e+02))
      (Variables|Default|Sethealth _output_get_5)
      (bind _output_get_6 (Variables|Default|SetMAX_MANA 75.0))
      (Variables|Default|Setmana _output_get_6))))

(fn GetWeapon
  (bind _asbase_sword (Utilities|Casting|CastToBaseSword (Variables|/Script/Engine.ChildActorComponent|GetChildActor (Variables|Default|GetWeapon))))
  (return _asbase_sword))