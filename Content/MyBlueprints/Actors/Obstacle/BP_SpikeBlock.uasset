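; BP_SpikeBlock is a spike trap obstacle that thrusts out when a damageable actor enters its trigger.
; After a configurable delay, MoveComponentTo eases the SpikeBlock component to a target relative location, waits briefly, then eases it back to the default zero offset.
; A separate Collision overlap damages any IDamageable actor and plays a hit sound, independent of the trap's movement state.
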(event OnComponentBeginOverlap(TriggerCollider)
  (params (OverlappedComponent :type Primitive%20Component%20Object%20Reference) (OtherActor :type Actor%20Object%20Reference) (OtherComp :type Primitive%20Component%20Object%20Reference) (OtherBodyIndex :type Integer) (bFromSweep :type Boolean) (SweepResult :type Hit%20Result%20Structure%20%28by%20ref%29))
  (bind _spikeblock (Variables|Default|GetSpikeBlock))
  ;[1 1 1] Trap actuation
  (Utilities|Casting|CastToIDamageable OtherActor)
  (Utilities|FlowControl|Delay (Variables|Default|GetTriggerDelay))
  (Components|MoveComponentTo _spikeblock (Variables|Default|GetTarget) "0, 0, 0" false true (Variables|Default|GetSpeed) false)
  (Utilities|FlowControl|Delay 2.5)
  (Components|MoveComponentTo _spikeblock "0, 0, 0" "0, 0, 0" false true 0.2 false))

(event OnComponentBeginOverlap(Collision)
  (params (OverlappedComponent :type Primitive%20Component%20Object%20Reference) (OtherActor :type Actor%20Object%20Reference) (OtherComp :type Primitive%20Component%20Object%20Reference) (OtherBodyIndex :type Integer) (bFromSweep :type Boolean) (SweepResult :type Hit%20Result%20Structure%20%28by%20ref%29))
  (bind _asidamageable (Utilities|Casting|CastToIDamageable OtherActor))
  (Default|GetDamaged _asidamageable (Variables|Default|GetDamage%20Amount))
  (Audio|PlaySoundatLocation (Variables|Default|GetHitSound) (Transformation|GetActorLocation) "0, 0, 0" 1.0 1.0 0.0 0 0 0))

(fn ConstructionScript)