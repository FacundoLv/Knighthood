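; Spike grate obstacle that cycles its spikes up and down and damages what touches it.
; On BeginPlay an endless FlipFlop and Delay loop eases the spikes between the Up and Down marker positions every StepDuration, with Invert swapping the phase.
; Overlapping the Collision component calls GetDamaged on actors implementing IDamageable and plays a hit sound at the grate.
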(event OnComponentBeginOverlap(Collision)
  (params (OverlappedComponent :type Primitive%20Component%20Object%20Reference) (OtherActor :type Actor%20Object%20Reference) (OtherComp :type Primitive%20Component%20Object%20Reference) (OtherBodyIndex :type Integer) (bFromSweep :type Boolean) (SweepResult :type Hit%20Result%20Structure%20%28by%20ref%29))
  (bind _asidamageable (Utilities|Casting|CastToIDamageable OtherActor))
  (Default|GetDamaged _asidamageable (Variables|Default|GetDamage))
  (Audio|PlaySoundatLocation (Variables|Default|GetHitSound) (Transformation|GetActorLocation) "0, 0, 0" 1.0 1.0 0.0 0 0 0))

(event EventBeginPlay
  (bind _invert (Variables|Default|GetInvert))
  ;[1 1 1] Back and forth movement
  (Utilities|FlowControl|FlipFlop :!label _label
    (:A
      (if _invert
        (Variables|Default|SetTarget (Variables|/Script/Engine.SceneComponent|GetRelativeLocation (Variables|Default|GetUp)) :!label _label_2)
        (else
          (Variables|Default|SetTarget (Variables|/Script/Engine.SceneComponent|GetRelativeLocation (Variables|Default|GetDown)) :!label _label_3))))
    (:B
      (if _invert
        (goto _label_3)
        (else
          (goto _label_2)))))
  (Components|MoveComponentTo (Variables|Default|GetSpikes) (Variables|Default|GetTarget) "0, 0, 0" false true 0.2 false)
  (Utilities|FlowControl|Delay (Variables|Default|GetStepDuration))
  (goto _label))

(event Collision|EventActorBeginOverlap
  (params (OtherActor :type Actor%20Object%20Reference)))

(event EventTick
  (params (DeltaSeconds :type Float%20%28single-precision%29)))

(fn ConstructionScript)