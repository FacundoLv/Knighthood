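; BP_BuzzSaw is a buzz saw obstacle that damages damageable actors on contact.
; A RotatingMovement component spins the Blade while BladeRoot eases endlessly between PointA and PointB, each leg lasting Cadence.
; A FlipFlop re-entered after each MoveComponentTo picks the next endpoint, and Invert swaps which point comes first.
; Collision overlaps apply DamageAmount through the IDamageable interface and play HitSound at the actor's location.
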(event OnComponentBeginOverlap(Collision)
  (params (OverlappedComponent :type Primitive%20Component%20Object%20Reference) (OtherActor :type Actor%20Object%20Reference) (OtherComp :type Primitive%20Component%20Object%20Reference) (OtherBodyIndex :type Integer) (bFromSweep :type Boolean) (SweepResult :type Hit%20Result%20Structure%20%28by%20ref%29))
  (bind _asidamageable (Utilities|Casting|CastToIDamageable OtherActor))
  (Default|GetDamaged _asidamageable (Variables|Default|GetDamage%20Amount))
  (Audio|PlaySoundatLocation (Variables|Default|GetHitSound) (Transformation|GetActorLocation) "0, 0, 0" 1.0 1.0 0.0 0 0 0))

(event EventBeginPlay
  (bind _invert (Variables|Default|GetInvert))
  (Components|Movement|SetUpdatedComponent (Variables|Default|GetRotatingMovement) (Variables|Default|GetBlade))
  ;[1 1 1] Back and forth movement
  (Utilities|FlowControl|FlipFlop :!label _label
    (:A
      (if _invert
        (Variables|Default|SetTarget (Variables|/Script/Engine.SceneComponent|GetRelativeLocation (Variables|Default|GetPointA)) :!label _label_2)
        (else
          (Variables|Default|SetTarget (Variables|/Script/Engine.SceneComponent|GetRelativeLocation (Variables|Default|GetPointB)) :!label _label_3))))
    (:B
      (if _invert
        (goto _label_3)
        (else
          (goto _label_2)))))
  (Components|MoveComponentTo (Variables|Default|GetBladeRoot) (Variables|Default|GetTarget) "0, 0, 0" true true (Variables|Default|GetCadence) false)
  (goto _label))

(fn ConstructionScript)