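; BP_MeleeHeavy is, by its name, a heavy melee enemy whose maximum health scales with game difficulty.
; SetEnemy reads CurrentDifficulty from KnighthoodGameInstance, raises MAXHEALTH from Easy through Normal to Hard, and sets Health to that maximum.
; The event graph holds only disabled stubs, and the construction script just calls its parent.
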(event EventBeginPlay
  (|CallParentFunction) ; This node is disabled and will not be called.\nDrag off pins to build functionality.
)

(event Collision|EventActorBeginOverlap
  (params (OtherActor :type Actor%20Object%20Reference))
  (|CallParentFunction OtherActor) ; This node is disabled and will not be called.\nDrag off pins to build functionality.
)

(event EventTick
  (params (DeltaSeconds :type Float%20%28single-precision%29))
  (|CallParentFunction DeltaSeconds) ; This node is disabled and will not be called.\nDrag off pins to build functionality.
)

(fn ConstructionScript
  (|CallParentFunction))

(fn SetEnemy
  (bind _asknighthood_game_instance (Utilities|Casting|CastToKnighthoodGameInstance (Game|GetGameInstance)))
  (switch Utilities|FlowControl|Switch|SwitchonGameDifficulty (Variables|/Game/MyBlueprints/KnighthoodGameInstance.KnighthoodGameInstance_C|GetCurrentDifficulty _asknighthood_game_instance)
    (:NewEnumerator0
      (bind _output_get (Variables|Default|SetMAX_HEALTH 1e+02))
      (Variables|Default|SetHealth _output_get))
    (:NewEnumerator1
      (bind _output_get_2 (Variables|Default|SetMAX_HEALTH 125.0))
      (Variables|Default|SetHealth _output_get_2))
    (:NewEnumerator2
      (bind _output_get_3 (Variables|Default|SetMAX_HEALTH 1.5e+02))
      (Variables|Default|SetHealth _output_get_3))))