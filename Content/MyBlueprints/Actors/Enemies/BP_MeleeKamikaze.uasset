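; Melee kamikaze enemy that attacks by blowing itself up near the player.
; Attack stops movement, plays the kamikaze montage and passes its length to OnExplode as the delay before the explosion effect and sound.
; The blast deals distance-scaled damage to the player within its radius, then destroys the actor and calls EnemyDown.
; SetEnemy sets blast radius and maximum damage from the game instance's difficulty.
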(event Custom|OnExplode
  (params (animDelay :type Float%20%28single-precision%29))
  (bind _returnvalue (Transformation|GetActorLocation))
  (bind _effectradius (Variables|Default|GetEffectRadius))
  (Utilities|FlowControl|Delay animDelay)
  (Effects|SpawnEmitteratLocation "/Game/PolygonKnights/ParticleFX/FX_Explosion.FX_Explosion" _returnvalue)
  (Audio|PlaySoundatLocation "/Game/MyActors/Sound/explosion.explosion" _returnvalue "0, 0, 0" 1.0 1.0 0.0 0 0 0)
  ;[1 1 1] Damage player based on distance and destroy self
  (bind _asbp_knighthood_character (Utilities|Casting|CastToBP_KnighthoodCharacter (Game|GetPlayerCharacter 0)))
  (if (<= (Transformation|GetDistanceTo _asbp_knighthood_character) _effectradius)
    (Default|GetDamaged _asbp_knighthood_character (Math|Float|MapRangeClamped (Transformation|GetDistanceTo _asbp_knighthood_character) _effectradius 0.0 0.0 (Variables|Default|GetMaxDamage))))
  (Actor|DestroyActor)
  (Default|CallEnemyDown))

(event EventBeginPlay
  (|CallParentFunction) ; This node is disabled and will not be called.\nDrag off pins to build functionality.
)

(fn ConstructionScript)

(fn SetEnemy
  (bind _asknighthood_game_instance (Utilities|Casting|CastToKnighthoodGameInstance (Game|GetGameInstance)))
  (switch Utilities|FlowControl|Switch|SwitchonGameDifficulty (Variables|/Game/MyBlueprints/KnighthoodGameInstance.KnighthoodGameInstance_C|GetCurrentDifficulty _asknighthood_game_instance)
    (:NewEnumerator0
      (Variables|Default|SetEffectRadius 2e+02)
      (Variables|Default|SetMaxDamage 75.0))
    (:NewEnumerator1
      (Variables|Default|SetEffectRadius 2e+02)
      (Variables|Default|SetMaxDamage 1e+02))
    (:NewEnumerator2
      (Variables|Default|SetEffectRadius 3e+02)
      (Variables|Default|SetMaxDamage 125.0))))

(fn Attack
  ;[1 1 1] Explode OnAttack
  (Class|NavMovementComponent|StopActiveMovement (Variables|Character|GetCharacterMovement))
  (bind _returnvalue (Animation|PlayAnimMontage (Variables|Default|GetKamikazeMontage) 1.0 "None"))
  (CallFunction|OnExplode _returnvalue)
  (return _returnvalue))