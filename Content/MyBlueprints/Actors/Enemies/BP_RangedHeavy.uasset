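; BP_RangedHeavy is an enemy actor Blueprint, named as a heavy ranged variant, that sets its damage from the game difficulty.
; SetEnemy reads CurrentDifficulty from KnighthoodGameInstance and assigns DamageAmount, with Easy and Normal sharing a value and Hard raising it.
; BeginPlay and the construction script only call the parent, and the file defines no attack or movement logic of its own.
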(event EventBeginPlay
  (|CallParentFunction))

(event Collision|EventActorBeginOverlap
  (params (OtherActor :type Actor%20Object%20Reference))
  (|CallParentFunction OtherActor) ; This node is disabled and will not be called.\nDrag off pins to build functionality.
)

(event EventTick
  (params (DeltaSeconds :type Float%20%28single-precision%29))
  (|CallParentFunction DeltaSeconds) ; This node is disabled and will not be called.\nDrag off pins to build functionality.
)

(fn ConstructionScript
  (|CallParentFunction))

(fn SetEnemy
  (bind _asknighthood_game_instance (Utilities|Casting|CastToKnighthoodGameInstance (Game|GetGameInstance)))
  (switch Utilities|FlowControl|Switch|SwitchonGameDifficulty (Variables|/Game/MyBlueprints/KnighthoodGameInstance.KnighthoodGameInstance_C|GetCurrentDifficulty _asknighthood_game_instance)
    (:NewEnumerator0
      (Variables|Default|SetDamage%20Amount 5e+01))
    (:NewEnumerator1
      (Variables|Default|SetDamage%20Amount 5e+01))
    (:NewEnumerator2
      (Variables|Default|SetDamage%20Amount 7e+01))))