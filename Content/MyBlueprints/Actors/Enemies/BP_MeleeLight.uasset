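; BP_MeleeLight is a light melee enemy character that carries a sword as a child actor and sets itself as its owner.
; On BeginPlay it scales max health by the game instance's difficulty and calls SetOrigin.
; Attack plays the attack montage and returns its duration, while GetWeapon exposes the child actor as a BaseSword.
; On death it plays a death montage, stops movement, and destroys itself after the montage's length.
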(event EventBeginPlay
  (CallFunction|SetEnemy)
  (CallFunction|SetOrigin))

(event EventOnDeath
  ;[1 1 1] OnDeath Behaviour
  (bind _returnvalue (Animation|PlayAnimMontage "/Game/MyActors/MyCharacter/AnimMontages/AM_Death.AM_Death" 1.0 "None"))
  (Class|NavMovementComponent|StopActiveMovement (Variables|Character|GetCharacterMovement))
  (Utilities|FlowControl|Delay _returnvalue)
  (Actor|DestroyActor))

(fn ConstructionScript
  (|CallParentFunction)
  (Actor|SetOwner (Variables|/Script/Engine.ChildActorComponent|GetChildActor (Variables|Default|GetWeapon)) self))

(fn SetEnemy
  (bind _asknighthood_game_instance (Utilities|Casting|CastToKnighthoodGameInstance (Game|GetGameInstance)))
  (switch Utilities|FlowControl|Switch|SwitchonGameDifficulty (Variables|/Game/MyBlueprints/KnighthoodGameInstance.KnighthoodGameInstance_C|GetCurrentDifficulty _asknighthood_game_instance)
    (:NewEnumerator0
      (bind _output_get (Variables|Default|SetMAX_HEALTH 75.0))
      (Variables|Default|SetHealth _output_get))
    (:NewEnumerator1
      (bind _output_get_2 (Variables|Default|SetMAX_HEALTH 1e+02))
      (Variables|Default|SetHealth _output_get_2))
    (:NewEnumerator2
      (bind _output_get_3 (Variables|Default|SetMAX_HEALTH 125.0))
      (Variables|Default|SetHealth _output_get_3))))

(fn Attack
  (bind _returnvalue (Animation|PlayAnimMontage (Variables|Default|GetAttackMontage) 1.0 "None"))
  (return _returnvalue))

(fn GetWeapon
  (bind _asbase_sword (Utilities|Casting|CastToBaseSword (Variables|/Script/Engine.ChildActorComponent|GetChildActor (Variables|Default|GetWeapon))))
  (return _asbase_sword))