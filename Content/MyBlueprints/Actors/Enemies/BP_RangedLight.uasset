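; BP_RangedLight is a ranged enemy that plays a cast animation to attack and fires projectiles.
; On BeginPlay it sets its origin and takes projectile damage from the game instance's difficulty, with only Hard differing.
; Attack only plays the montage; a separate OnShoot event spawns the SpellClass projectile at ShotDirection, passes on the damage and emits a gunshot effect.
; On death it stops movement, plays a death montage and destroys itself after the montage's length.
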(event Custom|OnShoot
  (bind _shotdirection (Variables|Default|GetShotDirection))
  (bind _returnvalue (Transformation|GetWorldLocation _shotdirection))
  (bind _returnvalue_2 (Transformation|GetWorldRotation _shotdirection))
  ;[1 1 1] Shooting behaviour
  (bind _asbase_projectile (Utilities|Casting|CastToBaseProjectileClass (Variables|Default|GetSpellClass)))
  (bind _returnvalue_3 (Game|SpawnActorfromClass _asbase_projectile (Math|Transform|MakeTransform _returnvalue _returnvalue_2 "1,1,1") "Undefined" self 0))
  (Variables|/Game/MyBlueprints/Actors/Weapons/BaseProjectile.BaseProjectile_C|SetDamage%20Amount _returnvalue_3 (Variables|Default|GetDamage%20Amount))
  (Effects|SpawnEmitteratLocation "/Game/PolygonKnights/ParticleFX/FX_Gunshot.FX_Gunshot" _returnvalue _returnvalue_2))

(event EventBeginPlay
  (CallFunction|SetEnemy)
  (CallFunction|SetOrigin))

(event EventOnDeath
  ;[1 1 1] OnDeath Behaviour
  (Class|NavMovementComponent|StopActiveMovement (Variables|Character|GetCharacterMovement))
  (bind _returnvalue (Animation|PlayAnimMontage (Variables|Default|GetDeathAnim) 1.0 "None"))
  (Utilities|FlowControl|Delay _returnvalue)
  (Actor|DestroyActor))

(fn ConstructionScript
  (|CallParentFunction))

(fn SetEnemy
  (bind _asknighthood_game_instance (Utilities|Casting|CastToKnighthoodGameInstance (Game|GetGameInstance)))
  (switch Utilities|FlowControl|Switch|SwitchonGameDifficulty (Variables|/Game/MyBlueprints/KnighthoodGameInstance.KnighthoodGameInstance_C|GetCurrentDifficulty _asknighthood_game_instance)
    (:NewEnumerator0
      (Variables|Default|SetDamage%20Amount 25.0))
    (:NewEnumerator1
      (Variables|Default|SetDamage%20Amount 25.0))
    (:NewEnumerator2
      (Variables|Default|SetDamage%20Amount 4e+01))))

(fn Attack
  (bind _returnvalue (Animation|PlayAnimMontage (Variables|Default|GetCastAnim) 1.0 "None"))
  (return _returnvalue))